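; Enemy melee attack gameplay ability that turns the avatar toward its combat target and plays a random tagged attack montage.
; The montage's tag serves as the gameplay event that triggers the hit and selects the combat socket location.
; A small sphere query there finds live players and damages non-friends.
; The ability ends after the hit or when the montage finishes or is interrupted, without stopping the montage.
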(event Ability|EventActivateAbility
  (bind _returnvalue (Ability|GetAvatarActorfromActorInfo))
  (bind _returnvalue_2 (Ability|GetAvatarActorfromActorInfo))
  (Development|PrintString "Hello")
  (bind _returnvalue_3 (Class|EnemyInterface|GetCombatTarget(Message) _returnvalue_2))
  (bind _asgame_combat_interface (Utilities|Casting|CastToGameCombatInterface _returnvalue_2))
  (Class|GameCombatInterface|UpdateFacingTarget _asgame_combat_interface (Transformation|GetActorLocation _returnvalue_3))
  (bind _returnvalue_4 (Class|GameCombatInterface|GetAttackMontages(Message) (Ability|GetAvatarActorfromActorInfo)))
  (bind _output_get (Variables|Default|SetTaggedMontage (Class|GameDamageGameplayAbility|GetRandomTaggedMontagefromArray _returnvalue_4)))
  (|PlayMontageandWaitProxy "None" (.Montage (Utilities|Struct|BreakTaggedMontage _output_get)) 1.0 "None" false 1.0 0.0
    (:then
      (Ability|Tasks|WaitGameplayEvent (.MontageTag (Utilities|Struct|BreakTaggedMontage _output_get)) 0
        (:EventReceived
          (bind _returnvalue_5 (Class|GameCombatInterface|GetCombatSocketLocation(Message) _returnvalue (.MontageTag (Utilities|Struct|BreakTaggedMontage _output_get))))
          (bind _outoverlappingactors (Class|GameAbilitySystemLibrary|GetLivePlayersWithinRadius _returnvalue (Utilities|Array|MakeArray _returnvalue) 45.0 _returnvalue_5))
          (for _array_element _outoverlappingactors
            (if (Class|GameAbilitySystemLibrary|IsNotFriend (Ability|GetAvatarActorfromActorInfo) _array_element)
              (Class|GameDamageGameplayAbility|CauseDamage _array_element)))
          (Ability|EndAbility))))
    (:OnCompleted
      (Ability|EndAbility :!label _label))
    (:OnInterrupted
      (goto _label))
    (:OnCancelled
      (goto _label))))

(event Ability|EventOnEndAbility
  (params (bWasCancelled :type Boolean)))